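; Cobweb wall actor that plays a death effect and removes itself once flagged as dead.
; Tick polls the Dead flag, which nothing in this graph sets, and makes five particle systems visible while it is true.
; A short Delay then runs before the actor destroys itself.
; The construction script is empty.
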(event `self.ReceiveTick`
  (params (DeltaSeconds :type "Float (single-precision)"))
  (if (`self.dead`)
    (`SceneComponent.SetVisibility` (`self.ParticleSystem`) true false)
    (`SceneComponent.SetVisibility` (`self.ParticleSystem1`) true false)
    (`SceneComponent.SetVisibility` (`self.ParticleSystem2`) true false)
    (`SceneComponent.SetVisibility` (`self.ParticleSystem3`) true false)
    (`SceneComponent.SetVisibility` (`self.ParticleSystem4`) true false)
    (`KismetSystemLibrary.Delay` 3.0)
    (`self.K2_DestroyActor`)))

(fn `UserConstructionScript`)