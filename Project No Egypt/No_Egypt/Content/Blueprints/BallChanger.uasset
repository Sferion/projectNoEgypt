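; BallChanger is a trigger actor that switches the ball's material type between wood, ice and fire, as set by its NewMat value.
; On BeginPlay, NewMat selects the center mesh's material and the matching color for its point light and spot light.
; When the player pawn overlaps it, it writes NewMat into BallMat on every Ball actor and spawns a scaled-up explosion near its center for each one.
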(event `self.ReceiveActorBeginOverlap`
  (params (OtherActor :type "Actor Object Reference"))
  (bind (_returnvalue_x _returnvalue_y _returnvalue_z) (`KismetMathLibrary.BreakVector` (`SceneComponent.K2_GetComponentLocation` (`self.Ball_changer_Center`))))
  (if (== OtherActor (`GameplayStatics.GetPlayerPawn` 0))
    (bind _outactors (`GameplayStatics.GetAllActorsOfClass` "/Game/Blueprints/Ball.Ball_C"))
    (for _array_element _outactors
      (set `/Game/Blueprints/Ball.ballMat` (`self.newMat`) _array_element)
      (`GameplayStatics.SpawnEmitterAtLocation` "/Game/StarterContent/Particles/P_Explosion.P_Explosion" (`KismetMathLibrary.MakeVector` (- _returnvalue_x 150.0) _returnvalue_y (+ _returnvalue_z 150.0)) (struct) (6.0 6.0 6.0)))))

(event `self.ReceiveBeginPlay`
  (bind _returnvalue (`KismetMathLibrary.Conv_VectorToLinearColor` (`self.fireColour`)))
  (bind _returnvalue_2 (`KismetMathLibrary.Conv_VectorToLinearColor` (`self.woodColour`)))
  (bind _returnvalue_3 (`KismetMathLibrary.Conv_VectorToLinearColor` (`self.iceColour`)))
  (if (== (`self.newMat`) 1)
    (`PrimitiveComponent.SetMaterial` (`self.Ball_changer_Center`) 0 "/Game/Materials/BallChanger_wood.BallChanger_wood")
    (`LightComponent.SetLightColor` (`self.PointLight`) _returnvalue_2 false)
    (`LightComponent.SetLightColor` (`self.SpotLight`) _returnvalue_2 false)
    (elif (== (`self.newMat`) 2)
      (`PrimitiveComponent.SetMaterial` (`self.Ball_changer_Center`) 0 "/Game/Materials/BallChanger_ice.BallChanger_ice")
      (`LightComponent.SetLightColor` (`self.PointLight`) _returnvalue_3 false)
      (`LightComponent.SetLightColor` (`self.SpotLight`) _returnvalue_3 false)
      (elif (== (`self.newMat`) 3)
        (`PrimitiveComponent.SetMaterial` (`self.Ball_changer_Center`) 0 "/Game/Materials/BallChanger_fire.BallChanger_fire")
        (`LightComponent.SetLightColor` (`self.PointLight`) _returnvalue false)
        (`LightComponent.SetLightColor` (`self.SpotLight`) _returnvalue false)))))

(fn `UserConstructionScript`)