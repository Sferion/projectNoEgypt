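; CamHeightSetter is a trigger volume that sets the CamHeight variable on every Ball actor while something overlaps its Box.
; Begin and end overlap events toggle an Overlapping flag without filtering which actor entered.
; While the flag is set, Tick finds all Balls each frame and writes NewHeight, or a fixed offset above the player pawn's Z position when NewHeight is zero.
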(event `self.Box.OnComponentBeginOverlap`
  (params (OverlappedComponent :type "PrimitiveComponent Object Reference") (OtherActor :type "Actor Object Reference") (OtherComp :type "PrimitiveComponent Object Reference") (OtherBodyIndex :type Integer) (bFromSweep :type Boolean) (SweepResult :type "HitResult Structure (by ref)"))
  (if true
    (set `self.overlapping` true)))

(event `self.Box.OnComponentEndOverlap`
  (params (OverlappedComponent :type "PrimitiveComponent Object Reference") (OtherActor :type "Actor Object Reference") (OtherComp :type "PrimitiveComponent Object Reference") (OtherBodyIndex :type Integer))
  (if true
    (set `self.overlapping` false)))

(event `self.ReceiveTick`
  (params (DeltaSeconds :type "Float (single-precision)"))
  (bind (_returnvalue_x _returnvalue_y _returnvalue_z) (`KismetMathLibrary.BreakVector` (`SceneComponent.K2_GetComponentLocation` (`Actor.RootComponent` (`GameplayStatics.GetPlayerPawn` 0)))))
  (if (`self.overlapping`)
    (if (== (`self.newHeight`) 0.0)
      (bind _outactors (`GameplayStatics.GetAllActorsOfClass` "/Game/Blueprints/Ball.Ball_C"))
      (for _array_element _outactors
        (set `/Game/Blueprints/Ball.camHeight` (+ _returnvalue_z 200.0) _array_element))
      (else
        (bind _outactors_2 (`GameplayStatics.GetAllActorsOfClass` "/Game/Blueprints/Ball.Ball_C"))
        (for _array_element_2 _outactors_2
          (set `/Game/Blueprints/Ball.camHeight` (`self.newHeight`) _array_element_2))))))

(fn `UserConstructionScript`)