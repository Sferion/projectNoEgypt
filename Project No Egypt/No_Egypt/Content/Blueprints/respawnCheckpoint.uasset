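; Respawn checkpoint actor that updates where Ball actors respawn while the player pawn is inside its trigger box.
; Box overlap events set an Overlapping flag for the player pawn.
; While the flag is set, Tick finds all Ball actors every frame and writes the checkpoint root's world location and rotation, plus StarterMat as default material, to each.
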(event `self.Box.OnComponentBeginOverlap`
  (params (OverlappedComponent :type "PrimitiveComponent Object Reference") (OtherActor :type "Actor Object Reference") (OtherComp :type "PrimitiveComponent Object Reference") (OtherBodyIndex :type Integer) (bFromSweep :type Boolean) (SweepResult :type "HitResult Structure (by ref)"))
  (if (== OtherActor (`GameplayStatics.GetPlayerPawn` 0))
    (set `self.overlapping` true)))

(event `self.Box.OnComponentEndOverlap`
  (params (OverlappedComponent :type "PrimitiveComponent Object Reference") (OtherActor :type "Actor Object Reference") (OtherComp :type "PrimitiveComponent Object Reference") (OtherBodyIndex :type Integer))
  (if (== OtherActor (`GameplayStatics.GetPlayerPawn` 0))
    (set `self.overlapping` false)))

(event `self.ReceiveTick`
  (params (DeltaSeconds :type "Float (single-precision)"))
  (bind _defaultsceneroot (`self.DefaultSceneRoot`))
  (if (`self.overlapping`)
    (bind _outactors (`GameplayStatics.GetAllActorsOfClass` "/Game/Blueprints/Ball.Ball_C"))
    (for _array_element _outactors
      (set `/Game/Blueprints/Ball.respawnLoc` (`SceneComponent.K2_GetComponentLocation` _defaultsceneroot) _array_element)
      (set `/Game/Blueprints/Ball.respawnRot` (`SceneComponent.K2_GetComponentRotation` _defaultsceneroot) _array_element)
      (set `/Game/Blueprints/Ball.defaultMat` (`self.starterMat`) _array_element))))

(fn `UserConstructionScript`)