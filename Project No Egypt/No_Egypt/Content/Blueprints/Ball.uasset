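; Player-controlled rolling ball that moves by physics torque from WASD keys, with a spring-arm camera.
; Each tick, BallMat selects concrete or wood, setting material, angular damping and torque strength, then held-key flags apply torque.
; The spring arm follows the ball horizontally at a height fixed on BeginPlay, and the mouse wheel zooms within limits.
; Mouse-look rotation nodes exist but are disconnected.
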(event `self.ReceiveBeginPlay`
  (bind (_returnvalue_x _returnvalue_y _returnvalue_z) (`KismetMathLibrary.BreakVector` (`SceneComponent.K2_GetComponentLocation` (`self.ball`))))
  (set `self.camHeight` (+ _returnvalue_z 200.0)))

(event `self.ReceiveTick`
  (params (DeltaSeconds :type "Float (single-precision)"))
  (bind _ball (`self.ball`))
  (bind _ball_2 (`self.ball`))
  (bind _returnvalue (`SceneComponent.K2_GetComponentLocation` _ball))
  (bind (_returnvalue_x _returnvalue_y) (`KismetMathLibrary.BreakVector` (`SceneComponent.K2_GetComponentLocation` (`self.ball`))))
  (if (== (`self.ballMat`) 0)
    (set `self.finalTorque` (`self.Torque`))
    (`PrimitiveComponent.SetMaterial` _ball_2 0 "/Game/StarterContent/Materials/M_Concrete_Tiles.M_Concrete_Tiles")
    (`PrimitiveComponent.SetAngularDamping` _ball_2 3.5)
    (elif (== (`self.ballMat`) 1)
      (set `self.finalTorque` (* (`self.Torque`) 2.5))
      (`PrimitiveComponent.SetMaterial` _ball_2 0 "/Game/StarterContent/Materials/M_Wood_Oak.M_Wood_Oak")
      (`PrimitiveComponent.SetAngularDamping` _ball_2 2.0)))
  (if (`self.wHeld`)
    (`PrimitiveComponent.AddTorqueInRadians` (`self.ball`) (`KismetMathLibrary.MakeVector` 0.0 (* (`self.finalTorque`) 5000000.0)) "None" false))
  (if (`self.sHeld`)
    (`PrimitiveComponent.AddTorqueInRadians` (`self.ball`) (`KismetMathLibrary.MakeVector` 0.0 (* (* (`self.finalTorque`) -1.0) 5000000.0)) "None" false))
  (if (`self.aHeld`)
    (`PrimitiveComponent.AddTorqueInRadians` (`self.ball`) (`KismetMathLibrary.MakeVector` (* (`self.finalTorque`) 5000000.0)) "None" false))
  (if (`self.dHeld`)
    (`PrimitiveComponent.AddTorqueInRadians` (`self.ball`) (`KismetMathLibrary.MakeVector` (* (* (`self.finalTorque`) -1.0) 5000000.0)) "None" false))
  (`SceneComponent.K2_SetWorldLocation` (`self.SpringArm`) (`KismetMathLibrary.MakeVector` _returnvalue_x _returnvalue_y (`self.camHeight`)) false false)
  (`SceneComponent.K2_SetWorldLocation` (`self.DefaultSceneRoot`) _returnvalue false false)
  (`SceneComponent.K2_SetWorldLocation` _ball _returnvalue false false))

(event `Key|W`
  (params (Key :type "Key Structure"))
  (:`Pressed`
    (set `self.wHeld` true))
  (:`Released`
    (set `self.wHeld` false)))

(event `Key|S`
  (params (Key :type "Key Structure"))
  (:`Pressed`
    (set `self.sHeld` true))
  (:`Released`
    (set `self.sHeld` false)))

(event `Key|A`
  (params (Key :type "Key Structure"))
  (:`Pressed`
    (set `self.aHeld` true))
  (:`Released`
    (set `self.aHeld` false)))

(event `Key|D`
  (params (Key :type "Key Structure"))
  (:`Pressed`
    (set `self.dHeld` true))
  (:`Released`
    (set `self.dHeld` false)))

(event `Key|MouseScrollUp`
  (params (Key :type "Key Structure"))
  (bind _springarm (`self.SpringArm`))
  (:`Pressed`
    (if (> (`SpringArmComponent.TargetArmLength` _springarm) 60.0)
      (set `SpringArmComponent.TargetArmLength` (+ (* (`self.zoomSpeed`) -1.0) (`SpringArmComponent.TargetArmLength` _springarm)) _springarm))))

(event `Key|MouseScrollDown`
  (params (Key :type "Key Structure"))
  (bind _springarm (`self.SpringArm`))
  (:`Pressed`
    (if (< (`SpringArmComponent.TargetArmLength` _springarm) 1200.0)
      (set `SpringArmComponent.TargetArmLength` (+ (`self.zoomSpeed`) (`SpringArmComponent.TargetArmLength` _springarm)) _springarm))))

(event `InputAxisKey|MouseY`
  (params (AxisValue :type "Float (single-precision)"))
  (if (!= AxisValue 0.0)
    _))

(event `InputAxisKey|MouseX`
  (params (AxisValue :type "Float (single-precision)"))
  (if (!= AxisValue 0.0)
    _))

(fn `UserConstructionScript`)