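; Ice bridge Blueprint whose cube disappears and stops colliding when flagged Dead, then regains collision after a delay.
; Tick polls Dead, which nothing in this file sets true, then hides the cube and disables collision for five seconds.
; It then clears Dead, enables query-only collision briefly, and restores physics collision if Dead is still false.
; The graph never makes the cube visible again.
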(event `self.ReceiveTick`
  (params (DeltaSeconds :type "Float (single-precision)"))
  (if (`self.dead`)
    (`SceneComponent.SetVisibility` (`self.Cube`) false false)
    (`PrimitiveComponent.SetCollisionEnabled` (`self.Cube`) "NoCollision")
    (`KismetSystemLibrary.Delay` 5.0)
    (set `self.dead` false)
    (`PrimitiveComponent.SetCollisionEnabled` (`self.Cube`) "QueryOnly")
    (`KismetSystemLibrary.Delay` 0.5)
    (if (not (`self.dead`))
      (`PrimitiveComponent.SetCollisionEnabled` (`self.Cube`) "QueryAndPhysics"))))

(fn `UserConstructionScript`)